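; Museum audio actor that switches ambient sound and music according to the player's camera view mode.
; BeginPlay caches the BP_PlayerCharacter, and Tick polls its CameraViewMode flag.
; When the flag is true it stops AmbientAudio and sets an '80s hero track on Music; when false it restarts ambience and sets the Kerala track.
; AmbientAudio's playing state gates each switch, so no separate state variable is kept.
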(event `self.ReceiveBeginPlay`
  (bind _returnvalue (`GameplayStatics.GetActorOfClass` "/Game/Blueprints/Player/BP_PlayerCharacter.BP_PlayerCharacter_C"))
  (set `self.As BP Player Character` _returnvalue))

(event `self.ReceiveTick`
  (params (DeltaSeconds :type "Float (single-precision)"))
  (if (`PlayerCharacter.CameraViewMode` (`self.As BP Player Character`))
    (if (`AudioComponent.IsPlaying` (`self.AmbientAudio`))
      (`AudioComponent.Stop` (`self.AmbientAudio`))
      (`AudioComponent.SetSound` (`self.Music`) "/Game/Audio/Origina/a-hero-of-the-80s-126684.a-hero-of-the-80s-126684"))
    (elif (not (`AudioComponent.IsPlaying` (`self.AmbientAudio`)))
      (`AudioComponent.Play` (`self.AmbientAudio`) 0.0)
      (`AudioComponent.SetSound` (`self.Music`) "/Game/Audio/Origina/kerala-113926.kerala-113926"))))

(fn `UserConstructionScript`)