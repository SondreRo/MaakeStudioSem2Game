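; Pawn for a tilt-the-ball minigame that unlocks a vault.
; Axis input rotates two components each tick, and a ball spawns on possession or respawns after falling too far below the pawn.
; When the ball overlaps the goal box, the first player character found is repossessed and the linked safe opens.
; Two hard-coded keys (Ø and X) trigger the same win flow directly.
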(event `Key|ø`
  (params (Key :type "Key Structure"))
  (:`Pressed`
    (bind _outactors (`GameplayStatics.GetAllActorsOfClass` "/Game/Blueprints/Player/BP_PlayerCharacter.BP_PlayerCharacter_C" :!label _label))
    (for _array_element _outactors
      (`Controller.Possess` (`GameplayStatics.GetPlayerController` 0) _array_element)
      (break))
    (`/Game/Blueprints/BP_Safe.OpenSafe` (`self.VaultToOpen`))))

(event `Won`
  (goto _label))

(event `self.ReceiveTick`
  (params (DeltaSeconds :type "Float (single-precision)"))
  (bind (_returnvalue_x _returnvalue_y _returnvalue_z) (`KismetMathLibrary.BreakVector` (`self.K2_GetActorLocation`)))
  (bind (_returnvalue_x_2 _returnvalue_y_2 _returnvalue_z_2) (`KismetMathLibrary.BreakVector` (`self.K2_GetActorLocation` (`self.Ball`))))
  (`SceneComponent.K2_AddRelativeRotation` (`self.XAxis`) (`KismetMathLibrary.MakeRotator` (`self.GetInputAxisKeyValue`)) false false)
  (`SceneComponent.K2_AddRelativeRotation` (`self.YAxis`) (`KismetMathLibrary.MakeRotator` 0.0 (* (`self.GetInputAxisKeyValue`) -1.0)) false false)
  (if (< _returnvalue_z_2 (- _returnvalue_z 600.0))
    (`self.K2_DestroyActor` (`self.Ball`))
    (`self.SpawnBall`)))

(event `self.ReceivePossessed`
  (params (NewController :type "Controller Object Reference"))
  (`/Engine/EditorBlueprintResources/StandardMacros.IsValid` (`self.Ball`) :!label _label_2
    (:`Is Not Valid`
      (if true
        (bind _returnvalue (`|SpawnActorFromClass` "/Game/Blueprints/Minigame/Ball.Ball_C" (`SceneComponent.K2_GetComponentToWorld` (`self.Spawn`)) "Undefined" "OverrideRootScale" null null))
        (set `self.Ball` _returnvalue)))))

(event `SpawnBall`
  (goto _label_2))

(event `self.Box.OnComponentBeginOverlap`
  (params (OverlappedComponent :type "PrimitiveComponent Object Reference") (OtherActor :type "Actor Object Reference") (OtherComp :type "PrimitiveComponent Object Reference") (OtherBodyIndex :type Integer) (bFromSweep :type Boolean) (SweepResult :type "HitResult Structure (by ref)"))
  (if (== OtherActor (`self.Ball`))
    (`self.Won` :!label _label_3)))

(event `Key|X`
  (params (Key :type "Key Structure"))
  (:`Pressed`
    (goto _label_3)))

(event `self.ReceiveUnpossessed`
  (params (OldController :type "Controller Object Reference")))

(fn `UserConstructionScript`)