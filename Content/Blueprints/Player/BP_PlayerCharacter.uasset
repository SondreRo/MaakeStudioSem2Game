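; Player character Blueprint that owns the player's HUD, held camera model visibility and menu hotkeys.
; BeginPlay creates core, interaction, trigger and task widgets into an AllHud array, shown on possession and hidden on unpossession, and caps frame rate via console command.
; Tick toggles the interaction prompt from CanInteract, while UpdateHand shows the camera model only for its item slot.
; Escape opens the main menu level; R pauses and shows a restart menu.
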(event `self.ReceiveBeginPlay`
  (bind _returnvalue (`GameplayStatics.GetPlayerController` 0))
  (`|ExecutionSequence`
    (:`then_0`
      (bind _returnvalue_2 (`|CreateWidget` "/Game/Blueprints/Hud/CoreHud.CoreHud_C" _returnvalue))
      (bind _output_get (set `self.CoreHud` _returnvalue_2))
      (`UserWidget.AddToViewport` _output_get 0)
      (`KismetArrayLibrary.Array_Add` (`self.AllHud`) _output_get))
    (:`then_1`
      (bind _returnvalue_3 (`|CreateWidget` "/Game/Blueprints/Hud/Interactions.Interactions_C" _returnvalue))
      (bind _output_get_2 (set `self.Interactions` _returnvalue_3))
      (`UserWidget.AddToViewport` _output_get_2 0)
      (`KismetArrayLibrary.Array_Add` (`self.AllHud`) _output_get_2))
    (:`then_2`
      (bind _returnvalue_4 (`|CreateWidget` "/Game/Blueprints/Hud/InteractionTrigger.InteractionTrigger_C" _returnvalue))
      (bind _output_get_3 (set `self.InteractionTrigger` _returnvalue_4))
      (`UserWidget.AddToViewport` _output_get_3 0)
      (`KismetArrayLibrary.Array_Add` (`self.AllHud`) _output_get_3))
    (:`then_3`
      (bind _returnvalue_5 (`|CreateWidget` "/Game/Blueprints/Hud/WB_Task.WB_Task_C" _returnvalue))
      (bind _output_get_4 (set `self.Tasks` _returnvalue_5))
      (`UserWidget.AddToViewport` _output_get_4 0)
      (`KismetArrayLibrary.Array_Add` (`self.AllHud`) _output_get_4))
    (:`then_4`
      (`KismetSystemLibrary.ExecuteConsoleCommand` "t.maxfps 100" null))))

(event `self.UpdateHand`
  (params (ItemSlot :type Integer))
  (`SceneComponent.SetHiddenInGame` (`self.CameraModel`) (!= ItemSlot 2) false))

(event `self.ReceiveTick`
  (params (DeltaSeconds :type "Float (single-precision)"))
  (bind _interactiontrigger (`self.InteractionTrigger`))
  (if (`self.CanInteract`)
    (`Widget.SetVisibility` _interactiontrigger "Visible")
    (else
      (`Widget.SetVisibility` _interactiontrigger "Collapsed"))))

(event `Key|Escape`
  (params (Key :type "Key Structure"))
  (:`Pressed`
    (`GameplayStatics.OpenLevelBySoftObjectPtr` "/Game/Levels/MainMenu.MainMenu")))

(event `self.ReceiveUnpossessed`
  (params (OldController :type "Controller Object Reference"))
  (for _array_element (`self.AllHud`)
    (`Widget.SetVisibility` _array_element "Collapsed")))

(event `Key|R`
  (params (Key :type "Key Structure"))
  (bind _returnvalue (`GameplayStatics.GetPlayerController` 0))
  (:`Pressed`
    (`GameplayStatics.SetGamePaused` true)
    (bind _returnvalue_2 (`|CreateWidget` "/Game/Blueprints/Hud/RestartMenu.RestartMenu_C" _returnvalue))
    (`UserWidget.AddToViewport` _returnvalue_2 0)
    (set `PlayerController.bShowMouseCursor` true _returnvalue)
    (`WidgetBlueprintLibrary.SetInputMode_GameOnly` (`GameplayStatics.GetPlayerController` 0))
    (`GameplayStatics.SetViewportMouseCaptureMode` "CapturePermanently_IncludingInitialMouseDown")))

(event `self.ReceivePossessed`
  (params (NewController :type "Controller Object Reference"))
  (for _array_element (`self.AllHud`)
    (`Widget.SetVisibility` _array_element "Visible")))

(fn `UserConstructionScript`)