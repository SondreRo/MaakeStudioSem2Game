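; BP_Safe is a safe hidden behind a painting that reveals a statue when opened.
; OpenSafe switches the player's view to the safe, enables collision on the statue, which is disabled at BeginPlay, and plays a timeline that slides the painting along Y.
; SoftReset moves the painting back to its origin but leaves the statue's collision unchanged.
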(event `self.ReceiveBeginPlay`
  (`self.SetActorEnableCollision` (`self.Statue`) false))

(event `OpenSafe`
  (`PlayerController.SetViewTargetWithBlend` (`GameplayStatics.GetPlayerController` 0) self 0.0 "VTBlend_Linear" 0.0 false)
  (`self.SetActorEnableCollision` (`self.Statue`) true)
  (bind (_direction _newtrack_0) (`Timeline|Timeline`)
    (:`Update`
      (`SceneComponent.K2_SetRelativeLocation` (`self.PaintingFixed`) (`KismetMathLibrary.MakeVector` 0.0 _newtrack_0) false false))))

(fn `SoftReset`
  (`SceneComponent.K2_SetRelativeLocation` (`self.PaintingFixed`) (0.0 0.0 0.0) false false))

(fn `UserConstructionScript`)